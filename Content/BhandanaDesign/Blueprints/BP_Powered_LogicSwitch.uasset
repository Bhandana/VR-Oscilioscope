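; BP_Powered_LogicSwitch is a voltage-gated switch that drives linked actors, apparently for unlocking doors.
; ShareVoltage compares incoming voltage to RequiredVoltage, turns the mesh green or red, and plays or reverses UnlockTimer.
; The timeline streams its percentage to every referenced actor through UpdateProgressMessage.
; The construction script starts it red with the requirement as text; its query functions report it as powered-type but supplying zero voltage.
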(event `/Game/BhandanaDesign/Blueprints/BPI_PowerSource.ShareVoltage`
  (params (Voltage :type "Float (single-precision)"))
  (bind _returnvalue (>= Voltage (`self.RequiredVoltage`)))
  ;[0.07996 0.1053 0.2865] Door Unlocking and Opening up
  (`MeshComponent.SetVectorParameterValueOnMaterials` (`self.StaticMesh`) "Colour" (`KismetMathLibrary.Conv_LinearColorToVector` (select `bool` _returnvalue :`false` (struct :`R` 1.0 :`B` 0.032916 :`A` 1.0) :`true` (struct :`G` 1.0 :`B` 0.100456 :`A` 1.0) :!type "LinearColor Structure")))
  (if _returnvalue
    (bind (_direction _percentage) (`Timeline|UnlockTimer` :!label _label)
      (:`Update`
        (for _array_element (`self.VAR_ActorReferences`)
          (message `/Game/BhandanaDesign/Blueprints/BPI_SpinGateSystem.UpdateProgress` _array_element _percentage))))
    (else
      (goto _label :!via `Reverse`))))

(fn `CheckifPoweredActor`
  (returns (`Is OSC` :type Boolean))
  (return true))

(fn `GetPairedAttachedActor`
  (returns (Actor :type "Actor Object Reference"))
  (return null))

(fn `GetVoltage`
  (returns (Voltage :type "Float (double-precision)"))
  (return 0.0))

(fn `UserConstructionScript`
  (`MeshComponent.SetVectorParameterValueOnMaterials` (`self.StaticMesh`) "Colour" (`KismetMathLibrary.Conv_LinearColorToVector` (struct :`R` 1.0 :`B` 0.032916 :`A` 1.0)))
  (`TextRenderComponent.K2_SetText` (`self.TextRender`) (`KismetTextLibrary.Conv_StringToText` (`KismetStringLibrary.Concat_StrStr` "Requires: " (`KismetStringLibrary.Conv_DoubleToString` (`self.RequiredVoltage`)) " Volts"))))