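; BP_Battery is a battery actor that holds a voltage value, apparently as a component of a power system.
; The construction script tints the model's materials with its Colour and writes the voltage to a text render label.
; Three query functions expose its state: GetVoltage returns PowerVoltage, CheckifPoweredActor always returns false and GetPairedAttachedActor returns without setting a result.
; It has no active runtime event logic.
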(fn `CheckifPoweredActor`
  (returns (`Is OSC` :type Boolean))
  (return false))

(fn `GetPairedAttachedActor`
  (returns (Actor :type "Actor Object Reference"))
  (return null))

(fn `GetVoltage`
  (returns (Voltage :type "Float (double-precision)"))
  (return (`self.PowerVoltage`)))

(fn `UserConstructionScript`
  (`parent.UserConstructionScript`)
  (`MeshComponent.SetVectorParameterValueOnMaterials` (`self.Model`) "Colour" (`KismetMathLibrary.Conv_LinearColorToVector` (`self.Colour`)))
  (`TextRenderComponent.K2_SetText` (`self.TextRender`) (`KismetTextLibrary.Conv_StringToText` (`KismetStringLibrary.Concat_StrStr` "Voltage: " (`KismetStringLibrary.Conv_DoubleToString` (`self.PowerVoltage`))))))