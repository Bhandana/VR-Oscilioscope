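; Inventory slot actor that accepts only listed item types and signals compatibility visually.
; InformInventorySlot colors SlotVisuals blue and enlarges it from the BeginPlay-saved scale for a match, red for a mismatch, and resets it without a valid actor.
; AssignItem hides the visuals and disables their overlaps when a valid item matches, without storing it.
; Accessory and attachment functions are empty stubs.
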(event `self.ReceiveBeginPlay`
  ;[0.07996 0.1053 0.2865] Saves the Size of the slot in memory
  (set `self.VAR_Scale_Memory` (`self.GetActorScale3D`)))

(fn `AssignAccessory`
  (params (ItemType :type "/Game/BhandanaDesign/Blueprints/ENUM_AttachmentTypes Enum" :default "NewEnumerator2") (`What we are assigning` :type "Actor Object Reference"))
  (returns (`Allowed in slot?` :type Boolean))
  (return false))

(fn `AssignItem`
  (params (ItemType :type "/Game/BhandanaDesign/Blueprints/ENUM_ItemTypes Enum" :default "NewEnumerator0") (`What we are assigning` :type "Actor Object Reference") (AttachmentType :type "/Game/BhandanaDesign/Blueprints/ENUM_AttachmentTypes Enum" :default "NewEnumerator2"))
  (returns (`Allowed in slot?` :type Boolean))
  (bind _slotvisuals (`self.SlotVisuals`))
  (bind _returnvalue (and (`self.CheckIfItemMatches` ItemType) (`KismetSystemLibrary.IsValid` `What we are assigning`)))
  (bind _returnvalue_2 (not _returnvalue))
  (set `PrimitiveComponent.bGenerateOverlapEvents` _returnvalue_2 _slotvisuals)
  (`SceneComponent.SetVisibility` _slotvisuals _returnvalue_2 false)
  (return _returnvalue))

(fn `CheckifHoldingAttachment`
  (returns (AttachmentMode :type Boolean) (`Types of attachments` :type "Array of /Game/BhandanaDesign/Blueprints/ENUM_AttachmentTypes Enum"))
  (return false))

(fn `CheckIfItemMatches`
  (params (ItemType :type "/Game/BhandanaDesign/Blueprints/ENUM_ItemTypes Enum" :default "NewEnumerator0"))
  (returns (Result :type Boolean))
  (locals (VAR_IsThereAMatch :type Boolean))
  (set `local.VAR_IsThereAMatch` false)
  (for _array_element (`self.VAR_AcceptedItemTypes`)
    (if (`|EnumEquality` _array_element ItemType)
      (set `local.VAR_IsThereAMatch` true)
      (break)))
  (return (`local.VAR_IsThereAMatch`)))

(fn `GetAttachmentTypes`
  (returns (AttachmentTypes :type "Array of /Game/BhandanaDesign/Blueprints/ENUM_AttachmentTypes Enum"))
  (return))

(fn `InformInventorySlot`
  (params (ItemType :type "/Game/BhandanaDesign/Blueprints/ENUM_ItemTypes Enum" :default "NewEnumerator0") (Actor :type "Actor Object Reference") (AttachmentTypes :type "/Game/BhandanaDesign/Blueprints/ENUM_AttachmentTypes Enum" :default "NewEnumerator2"))
  (returns (`Allowed in slot?` :type Boolean))
  (bind _result (`self.CheckIfItemMatches` ItemType))
  (`/Engine/EditorBlueprintResources/StandardMacros.IsValid` Actor
    (:`Is Valid`
      (`SceneComponent.SetWorldScale3D` (`self.SlotVisuals`) (select `bool` _result :`false` (`self.VAR_Scale_Memory`) :`true` (* (`self.VAR_Scale_Memory`) 1.25)))
      (`MeshComponent.SetVectorParameterValueOnMaterials` (`self.SlotVisuals`) "BaseColor" (`KismetMathLibrary.Conv_LinearColorToVector` (select `bool` _result :`false` (struct :`R` 1.0 :`B` 0.032916 :`A` 1.0) :`true` (struct :`R` 0.066176 :`G` 0.210765 :`B` 0.295 :`A` 1.0) :!type "LinearColor Structure")))
      (return _result))
    (:`Is Not Valid`
      (`SceneComponent.SetWorldScale3D` (`self.SlotVisuals`) (`self.VAR_Scale_Memory`))
      (`MeshComponent.SetVectorParameterValueOnMaterials` (`self.SlotVisuals`) "BaseColor" (`KismetMathLibrary.Conv_LinearColorToVector` (struct :`R` 0.066176 :`G` 0.210765 :`B` 0.295 :`A` 1.0)))
      (return (`self.CheckIfItemMatches` ItemType)))))

(fn `UserConstructionScript`)