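; Oscilloscope (OSC) actor that displays received voltages on up to four channels through material parameters on its mesh.
; The construction script gathers child inventory slots as channels, and a slot check sets the active channel by that slot's index.
; Shared voltage is printed, scaled down and written to the active channel's parameter.
; A Power interact request flips the material's power parameter.
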(event `/Game/BhandanaDesign/Blueprints/BPI_PowerSource.ShareVoltage`
  (params (Voltage :type "Float (single-precision)"))
  (`KismetSystemLibrary.PrintString` (`KismetStringLibrary.Concat_StrStr` "The OSC recieeived a voltage of: " (`KismetStringLibrary.Conv_DoubleToString` Voltage)) true true (struct :`R` 1.0 :`B` 0.032916 :`A` 1.0))
  (`MeshComponent.SetScalarParameterValueOnMaterials` (`self.StaticMeshComponent`) (select `int` (`self.Var_ActiveChannel`) :`0` "Voltage1" :`1` "Voltage2" :`2` "Voltage3" :`3` "Voltage4" :!type "Name") (/ Voltage 10.0)))

(event `TogglePower`
  (bind _isa (`/Engine/EditorBlueprintResources/StandardMacros.FlipFlop`)
    (:`A`
      _)
    (:`B`
      _))
  (`MeshComponent.SetScalarParameterValueOnMaterials` (`self.StaticMeshComponent`) "Power" (select `bool` _isa :`true` 1.0 :!type "Float (single-precision)")))

(event `/Game/BhandanaDesign/Blueprints/BPI_Interactions.InteractRequest`
  (params (`Request tag` :type Name))
  (switch `name` `Request tag`
    (:`Power`
      (`self.TogglePower`))))

(event `/Game/BhandanaDesign/Blueprints/BPI_PowerSource.OSCCheckChannel`
  (params (SlotCheck :type "Actor Object Reference"))
  (for (_array_element _array_index) (`self.VAR_ChannelList`)
    (if (== _array_element SlotCheck)
      (set `self.Var_ActiveChannel` _array_index)
      (break))))

(fn `CheckifOSC`
  (returns (`Is OSC` :type Boolean))
  (return true))

(fn `GetPairedAttachedActor`
  (returns (Actor :type "Actor Object Reference"))
  (return null))

(fn `GetVoltage`
  (returns (Voltage :type "Float (double-precision)"))
  (return 0.0))

(fn `UserConstructionScript`
  (`KismetArrayLibrary.Array_Clear` (`self.VAR_ChannelList`))
  (for _array_element (`self.GetAllChildActors` true)
    (if (== (`GameplayStatics.GetObjectClass` _array_element) "/Game/BhandanaDesign/Blueprints/BP_InventorySlot.BP_InventorySlot_C")
      (`KismetArrayLibrary.Array_Add` (`self.VAR_ChannelList`) _array_element))))