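; BP_Item is a grabbable item that BP_MotionController can pick up and that can be stored in inventory slots.
; Overlaps with Inventory-tagged actors record a candidate slot through interface messages.
; Pickup attaches it to the hand and clears its old slot, while Drop snaps it into an accepting slot or restores physics.
; On BeginPlay it spawns and attaches either preset attachments or BP_AttachmentSlot actors from its AttachmentSlots array.
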(event `self.Model.OnComponentBeginOverlap`
  (params (OverlappedComponent :type "PrimitiveComponent Object Reference") (OtherActor :type "Actor Object Reference") (OtherComp :type "PrimitiveComponent Object Reference") (OtherBodyIndex :type Integer) (bFromSweep :type Boolean) (SweepResult :type "HitResult Structure (by ref)"))
  ;[0.07996 0.1053 0.2865] Stores the Actor in memory if it's an inventory slot, and checks if the item can go there
  (if (and (`self.ActorHasTag` OtherActor "Inventory") (`self.VAR_IsHeld`))
    (bind _allowed_in_slot_ (message `/Game/BhandanaDesign/Blueprints/BPI_InventorySystem.InformInventorySlot` OtherActor (`self.ItemType`) self (`self.AttachmentType`)))
    (if _allowed_in_slot_
      (set `self.SlotActorReference` OtherActor))))

(event `/Game/VirtualRealityBP/Blueprints/PickupActorInterface.Pickup`
  (params (AttachTo :type "SceneComponent Object Reference"))
  (bind _returnvalue (select `bool` (`self.VAR_IsSnapToTarget`) :`false` "KeepWorld" :`true` "SnapToTarget" :!type "EAttachmentRule Enum"))
  ;[0.07996 0.1053 0.2865] Attaches the actor to the hand that grabbed it; Updates the inventory slot it came from (if it did)
  (set `self.VAR_IsHeld` true)
  (`/Engine/EditorBlueprintResources/StandardMacros.IsValid` (`self.SlotActorReferenceMemory`)
    (:`Is Valid`
      (message `/Game/BhandanaDesign/Blueprints/BPI_InventorySystem.AssignItem` (`self.SlotActorReferenceMemory`) (`self.ItemType`) null "NewEnumerator0")
      (set `self.SlotActorReferenceMemory` null))
    (:`Is Not Valid`
      _))
  (`PrimitiveComponent.SetSimulatePhysics` (`self.Model`) false)
  (`SceneComponent.K2_AttachToComponent` (`self.K2_GetRootComponent`) AttachTo "None" _returnvalue _returnvalue "KeepWorld" false)
  (`PrimitiveComponent.SetCollisionResponseToChannel` (`self.Model`) "ECC_Visibility" "ECR_Ignore"))

(event `self.Model.OnComponentEndOverlap`
  (params (OverlappedComponent :type "PrimitiveComponent Object Reference") (OtherActor :type "Actor Object Reference") (OtherComp :type "PrimitiveComponent Object Reference") (OtherBodyIndex :type Integer))
  ;[0.07996 0.1053 0.2865] Clears the reference of which slot this item is overlapping, when it leaves that slot's area
  (if (`self.ActorHasTag` OtherActor "Inventory")
    (bind _allowed_in_slot_ (message `/Game/BhandanaDesign/Blueprints/BPI_InventorySystem.InformInventorySlot` OtherActor (`self.ItemType`) null (`self.AttachmentType`)))
    (if (and _allowed_in_slot_ (== (`self.SlotActorReference`) OtherActor))
      (set `self.SlotActorReference` null))))

(event `self.ReceiveBeginPlay`
  ;[0.07996 0.1053 0.2865] Begin Play -- Sets the scale to Absolute so inventory slots don't mess with it
  (`self.CreateAttachments`)
  (`SceneComponent.SetAbsolute` (`self.Model`) false false true))

(event `/Game/VirtualRealityBP/Blueprints/PickupActorInterface.Drop`
  (bind _model (`self.Model`))
  (bind _slotactorreference (`self.SlotActorReference`))
  ;[0.07996 0.1053 0.2865] Drops the item, putting it into a slot if it's intended to go into one.
  (set `self.VAR_IsHeld` false)
  (`/Engine/EditorBlueprintResources/StandardMacros.IsValid` _slotactorreference
    (:`Is Valid`
      (if (!= (`self.GetParentActor` _slotactorreference) self)
        (`SceneComponent.K2_AttachToComponent` (`self.K2_GetRootComponent`) (`Actor.RootComponent` (`self.SlotActorReference`)) "None" "SnapToTarget" "SnapToTarget" "KeepWorld" false)
        (`self.K2_AddActorLocalRotation` (`SceneComponent.RelativeRotation` (`self.InventoryRotation`)))
        (set `self.SlotActorReferenceMemory` (`self.SlotActorReference`))
        (bind _allowed_in_slot_ (message `/Game/BhandanaDesign/Blueprints/BPI_InventorySystem.AssignItem` (`self.SlotActorReference`) (`self.ItemType`) self (`self.AttachmentType`)))
        (if _allowed_in_slot_
          (`PrimitiveComponent.SetCollisionResponseToChannel` _model "ECC_Visibility" "ECR_Ignore")
          (`PrimitiveComponent.SetCollisionEnabled` _model "QueryOnly")
          (else
            (`self.ManualDrop`)
            (set `self.SlotActorReferenceMemory` null)))
        (else
          (`PrimitiveComponent.SetSimulatePhysics` (`self.Model`) true :!label _label)
          (`self.K2_DetachFromActor` "KeepWorld" "KeepWorld" "KeepWorld")
          (`PrimitiveComponent.SetCollisionResponseToChannel` (`self.Model`) "ECC_Visibility" "ECR_Block")
          (`PrimitiveComponent.SetCollisionEnabled` (`self.Model`) "QueryAndPhysics")
          (set `self.SlotActorReference` null)
          (set `self.SlotActorReferenceMemory` null))))
    (:`Is Not Valid`
      (goto _label))))

(event `ManualDrop`
  ;[0.07996 0.1053 0.2865] Drops the item, putting it into a slot if it's intended to go into one.
  (goto _label))

(fn `AssignAccessory`
  (params (ItemType :type "/Game/BhandanaDesign/Blueprints/ENUM_AttachmentTypes Enum" :default "NewEnumerator2") (`What we are assigning` :type "Actor Object Reference"))
  (returns (`Allowed in slot?` :type Boolean))
  (return false))

(fn `AssignItem`
  (params (ItemType :type "/Game/BhandanaDesign/Blueprints/ENUM_ItemTypes Enum" :default "NewEnumerator0") (`What we are assigning` :type "Actor Object Reference") (AttachmentType :type "/Game/BhandanaDesign/Blueprints/ENUM_AttachmentTypes Enum" :default "NewEnumerator2"))
  (returns (`Allowed in slot?` :type Boolean))
  (return false))

(fn `CheckifHoldingAttachment`
  (returns (AttachmentMode :type Boolean) (`Types of attachments` :type "Array of /Game/BhandanaDesign/Blueprints/ENUM_AttachmentTypes Enum"))
  (return false))

(fn `CreateAttachments`
  ;[1 0 0.03292] Adds the attachment slots for the item, based on if it needs any
  (for _array_element (`self.Attachment Slots`)
    (bind (_isoccupied _attachmenttransform _typeofattachmentsallowed _attachedobject) (break `/Game/BhandanaDesign/Blueprints/STRUCT_AttachPoint` _array_element))
    (if (`KismetSystemLibrary.IsValidClass` _attachedobject)
      (bind _returnvalue (`|SpawnActorFromClass` _attachedobject _attachmenttransform "Undefined" "OverrideRootScale" null "NewEnumerator2" null))
      (`self.K2_AttachToActor` _returnvalue self "None" "KeepRelative" "KeepRelative" "KeepRelative" true)
      (`self.K2_SetActorRelativeTransform` _returnvalue _attachmenttransform false true)
      (else
        (bind _returnvalue_2 (`|SpawnActorFromClass` "/Game/BhandanaDesign/Blueprints/BP_AttachmentSlot.BP_AttachmentSlot_C" _attachmenttransform "Undefined" "OverrideRootScale" null _typeofattachmentsallowed null))
        (`self.K2_AttachToActor` _returnvalue_2 self "None" "KeepRelative" "KeepRelative" "KeepRelative" true)
        (`self.K2_SetActorRelativeTransform` _returnvalue_2 _attachmenttransform false true)))))

(fn `GetAttachmentTypes`
  (returns (AttachmentTypes :type "Array of /Game/BhandanaDesign/Blueprints/ENUM_AttachmentTypes Enum"))
  (locals (AcceptedAttachments :type "Array of /Game/BhandanaDesign/Blueprints/ENUM_AttachmentTypes Enum"))
  ;[0.06618 0.2108 0.295] Returns what types of attachments are allowed into each slot, if any
  (`KismetArrayLibrary.Array_Clear` (`local.AcceptedAttachments`))
  (for _array_element (`self.Attachment Slots`)
    (bind (_isoccupied _attachmenttransform _typeofattachmentsallowed) (break `/Game/BhandanaDesign/Blueprints/STRUCT_AttachPoint` _array_element))
    (if (not _isoccupied)
      (`KismetArrayLibrary.Array_Append` (`local.AcceptedAttachments`) _typeofattachmentsallowed)))
  (return (`local.AcceptedAttachments`)))

(fn `InformInventorySlot`
  (params (ItemType :type "/Game/BhandanaDesign/Blueprints/ENUM_ItemTypes Enum" :default "NewEnumerator0") (Actor :type "Actor Object Reference") (AttachmentTypes :type "/Game/BhandanaDesign/Blueprints/ENUM_AttachmentTypes Enum" :default "NewEnumerator2"))
  (returns (`Allowed in slot?` :type Boolean))
  (return false))

(fn `UserConstructionScript`)