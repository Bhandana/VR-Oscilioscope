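; Interactive oscilloscope device that shows received voltages on its screen material across up to four channels.
; Construction script gathers child BP_InventorySlot actors as channels, and OSCCheckChannel makes the matching slot the active channel.
; ShareVoltage writes scaled voltage to that channel's scalar material parameter.
; A Power interaction flip-flops the screen and button colour from a default off state; CheckifPoweredActor always returns true, regardless of that state.
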(event `self.ReceiveBeginPlay`
  ;[1 0 0.03292] Begin play: Defaults the display to be powered off
  (message `/Game/BhandanaDesign/Blueprints/BPI_Interactions.UpdateColour` (`self.PowerButton`) (struct :`R` 1.0 :`B` 0.032916 :`A` 1.0))
  (`MeshComponent.SetScalarParameterValueOnMaterials` (`self.StaticMeshComponent`) "Power" 0.0))

(event `TogglePower`
  ;[0.07996 0.1053 0.2865] Toggles the power button on the Oscilloscope, which impacts the display on it's screen material
  (bind _isa (`/Engine/EditorBlueprintResources/StandardMacros.FlipFlop`)
    (:`A`
      _)
    (:`B`
      _))
  (`MeshComponent.SetScalarParameterValueOnMaterials` (`self.StaticMeshComponent`) "Power" (select `bool` _isa :`true` 1.0 :!type "Float (single-precision)"))
  (message `/Game/BhandanaDesign/Blueprints/BPI_Interactions.UpdateColour` (`self.PowerButton`) (select `bool` _isa :`false` (struct :`R` 1.0 :`B` 0.032916 :`A` 1.0) :`true` (struct :`G` 1.0 :`B` 0.100456 :`A` 1.0) :!type "LinearColor Structure")))

(event `/Game/BhandanaDesign/Blueprints/BPI_PowerSource.ShareVoltage`
  (params (Voltage :type "Float (single-precision)"))
  ;[0.07996 0.1053 0.2865] Reads the power data given to the Oscilloscope, and updates it's material accordingly
  (`MeshComponent.SetScalarParameterValueOnMaterials` (`self.StaticMeshComponent`) (select `int` (`self.Var_ActiveChannel`) :`0` "Voltage1" :`1` "Voltage2" :`2` "Voltage3" :`3` "Voltage4" :!type "Name") (/ Voltage 10.0)))

(event `/Game/BhandanaDesign/Blueprints/BPI_PowerSource.OSCCheckChannel`
  (params (SlotCheck :type "Actor Object Reference"))
  ;[0.06618 0.2108 0.295] Checks if the cable actor is plugged into one this this Oscilloscope's channels, and sets that channel to the Active Channel Interval
  (for (_array_element _array_index) (`self.VAR_ChannelList`)
    (if (== _array_element SlotCheck)
      (set `self.Var_ActiveChannel` _array_index)
      (break))))

(event `/Game/BhandanaDesign/Blueprints/BPI_Interactions.InteractRequest`
  (params (`Request tag` :type Name))
  ;[0.06618 0.2108 0.295] Main Interaction handler, when the type of action by name matches, the repsective event will be fired
  (switch `name` `Request tag`
    (:`Power`
      (`self.TogglePower`))))

(fn `CheckifPoweredActor`
  (returns (`Is OSC` :type Boolean))
  (return true))

(fn `GetPairedAttachedActor`
  (returns (Actor :type "Actor Object Reference"))
  (return null))

(fn `GetVoltage`
  (returns (Voltage :type "Float (double-precision)"))
  (return 0.0))

(fn `UserConstructionScript`
  ;[0.06618 0.2108 0.295] Builds the list of child actors which are used to control channels
  (`KismetArrayLibrary.Array_Clear` (`self.VAR_ChannelList`))
  (for _array_element (`self.GetAllChildActors` true)
    (if (== (`GameplayStatics.GetObjectClass` _array_element) "/Game/BhandanaDesign/Blueprints/Inventory/BP_InventorySlot.BP_InventorySlot_C")
      (`KismetArrayLibrary.Array_Add` (`self.VAR_ChannelList`) _array_element))))