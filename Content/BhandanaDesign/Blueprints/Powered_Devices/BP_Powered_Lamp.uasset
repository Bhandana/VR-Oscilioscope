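; BP_Powered_Lamp is a powered-device lamp whose brightness follows its stored voltage.
; UpdatePowerBehaviors scales the SpotLight intensity and the Bulb material's Glow_Intensity parameter from that voltage, and also runs on BeginPlay to set the initial look.
; It identifies itself as a powered actor through CheckifPoweredActor and leaves voltage sharing to its parent class.
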(event `self.ReceiveBeginPlay`
  (`self.Update Power Behaviors`))

(event `/Game/BhandanaDesign/Blueprints/BPI_PowerSource.ShareVoltage`
  (params (Voltage :type "Float (single-precision)"))
  (`parent.ShareVoltage` Voltage))

(event `self.Update Power Behaviors`
  (`LightComponent.SetIntensity` (`self.SpotLight`) (* 100 (`self.VAR_Stored Voltage`)))
  (`MeshComponent.SetScalarParameterValueOnMaterials` (`self.Bulb`) "Glow_Intensity" (/ (`self.VAR_Stored Voltage`) 100.0)))

(fn `CheckifPoweredActor`
  (returns (`Is OSC` :type Boolean))
  (return true))

(fn `UserConstructionScript`
  (`parent.UserConstructionScript`))