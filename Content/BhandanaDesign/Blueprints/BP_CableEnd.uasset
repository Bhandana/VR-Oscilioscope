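; Pickup-and-drop cable end that pairs with another end to carry voltage between devices it plugs into.
; The host end builds a visible cable component to its pair in construction, and BeginPlay adds a physics constraint, noted as breaking once plugged in.
; Drop reads voltage from BPI_PowerSource slot owners, shares it with the pair and attached devices, and triggers their OSC channel checks.
; Pickup zeroes voltage to a connected powered device.
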(event `self.ReceiveBeginPlay`
  (bind (_returnvalue_location _returnvalue_rotation) (`KismetMathLibrary.BreakTransform` (`SceneComponent.GetRelativeTransform` (`self.Model`))))
  ;[1 0 0.03292] Builds physics for the cable, not fully functioning at the moment; Needs improvements due to physics breaking once plugged in
  (`parent.ReceiveBeginPlay`)
  (`/Engine/EditorBlueprintResources/StandardMacros.IsValid` (`self.Cable-Pair_Reference`)
    (:`Is Valid`
      (bind _returnvalue (`AddComponent|NODE_AddPhysicsConstraintComponent-1` :`RelativeTransform` (`KismetMathLibrary.MakeTransform` _returnvalue_location _returnvalue_rotation)))
      (`PhysicsConstraintComponent.SetConstrainedComponents` _returnvalue (`self.Model`) "None" (`self.GetComponentByClass` (`self.Cable-Pair_Reference`) "/Script/Engine.StaticMeshComponent") "None"))))

(event `/Game/BhandanaDesign/Blueprints/BPI_PowerSource.ShareVoltage`
  (params (Voltage :type "Float (single-precision)"))
  ;[1 1 1] Gets the partner cable's updated power settings, and stores them into a variable
  (set `self.Pair_Voltage_Memory` Voltage))

(event `/Game/VirtualRealityBP/Blueprints/PickupActorInterface.Drop`
  (bind _slotactorreferencememory (`self.SlotActorReferenceMemory`))
  (bind _cable_pair_reference (`self.Cable-Pair_Reference`))
  (bind _returnvalue (`self.GetParentActor` _slotactorreferencememory))
  ;[0.07996 0.1053 0.2865] Collects Voltage data from the actor this cable gets plugged into, if any, and informs the other all actors involved of the updated power settings.
  (`parent.Drop`)
  (`/Engine/EditorBlueprintResources/StandardMacros.IsValid` _slotactorreferencememory
    (:`Is Valid`
      (if (`KismetSystemLibrary.DoesImplementInterface` _returnvalue "/Game/BhandanaDesign/Blueprints/BPI_PowerSource.BPI_PowerSource_C")
        (`|ExecutionSequence`
          (:`then_0`
            (bind _voltage (message `/Game/BhandanaDesign/Blueprints/BPI_PowerSource.GetVoltage` _returnvalue))
            (bind _output_get (set `self.Voltage_Memory` _voltage))
            (message `/Game/BhandanaDesign/Blueprints/BPI_PowerSource.ShareVoltage` _cable_pair_reference _output_get)
            (bind _actor (message `/Game/BhandanaDesign/Blueprints/BPI_PowerSource.GetPairedAttachedActor` _cable_pair_reference))
            (`/Engine/EditorBlueprintResources/StandardMacros.IsValid` _actor
              (:`Is Valid`
                (bind _returnvalue_2 (`self.GetParentActor` _actor))
                (`/Engine/EditorBlueprintResources/StandardMacros.IsValid` _returnvalue_2
                  (:`Is Valid`
                    (message `/Game/BhandanaDesign/Blueprints/BPI_PowerSource.OSCCheckChannel` _returnvalue_2 _actor)
                    (message `/Game/BhandanaDesign/Blueprints/BPI_PowerSource.ShareVoltage` _returnvalue_2 (`self.Voltage_Memory`)))))))
          (:`then_1`
            (message `/Game/BhandanaDesign/Blueprints/BPI_PowerSource.OSCCheckChannel` _returnvalue (`self.SlotActorReferenceMemory`))
            (message `/Game/BhandanaDesign/Blueprints/BPI_PowerSource.ShareVoltage` _returnvalue (`self.Pair_Voltage_Memory`))))
        (else
          (set `self.Voltage_Memory` 0.0 :!label _label))))
    (:`Is Not Valid`
      (goto _label))))

(event `/Game/VirtualRealityBP/Blueprints/PickupActorInterface.Pickup`
  (params (AttachTo :type "SceneComponent Object Reference"))
  (bind _slotactorreferencememory (`self.SlotActorReferenceMemory`))
  (bind _returnvalue (`self.GetParentActor` _slotactorreferencememory))
  ;[0.07996 0.1053 0.2865] Updates power settings accordingly, and shuts off power going to any devices that were involved with the cables.
  (set `self.Voltage_Memory` 0.0)
  (`/Engine/EditorBlueprintResources/StandardMacros.IsValid` (`self.Cable-Pair_Reference`)
    (:`Is Valid`
      (`/Engine/EditorBlueprintResources/StandardMacros.IsValid` _slotactorreferencememory
        (:`Is Valid`
          (bind _actor (message `/Game/BhandanaDesign/Blueprints/BPI_PowerSource.GetPairedAttachedActor` (`self.Cable-Pair_Reference`)))
          (`/Engine/EditorBlueprintResources/StandardMacros.IsValid` _actor
            (:`Is Valid`
              (bind _returnvalue_2 (`self.GetParentActor` _actor))
              (bind _is_osc (message `/Game/BhandanaDesign/Blueprints/BPI_PowerSource.CheckifPoweredActor` _returnvalue_2))
              (bind _is_osc_2 (message `/Game/BhandanaDesign/Blueprints/BPI_PowerSource.CheckifPoweredActor` _returnvalue))
              (if (or _is_osc_2 _is_osc)
                (bind _returnvalue_3 (select `bool` _is_osc_2 :`false` _returnvalue_2 :`true` _returnvalue))
                (message `/Game/BhandanaDesign/Blueprints/BPI_PowerSource.OSCCheckChannel` _returnvalue_3 (select `bool` _is_osc_2 :`false` _actor :`true` (`self.SlotActorReferenceMemory`)))
                (message `/Game/BhandanaDesign/Blueprints/BPI_PowerSource.ShareVoltage` _returnvalue_3 0.0))
              (`parent.Pickup` AttachTo))
            (:`Is Not Valid`
              (`parent.Pickup` AttachTo :!label _label_2))))
        (:`Is Not Valid`
          (goto _label_2))))
    (:`Is Not Valid`
      (goto _label_2))))

(fn `CheckifPoweredActor`
  (returns (`Is OSC` :type Boolean))
  (return false))

(fn `GetPairedAttachedActor`
  (returns (Actor :type "Actor Object Reference"))
  (bind _slotactorreferencememory (`self.SlotActorReferenceMemory`))
  (`/Engine/EditorBlueprintResources/StandardMacros.IsValid` _slotactorreferencememory
    (:`Is Valid`
      (return _slotactorreferencememory))
    (:`Is Not Valid`
      (return null))))

(fn `GetVoltage`
  (returns (Voltage :type "Float (double-precision)"))
  (return 0.0))

(fn `UserConstructionScript`
  (bind _cable_pair_reference (`self.Cable-Pair_Reference`))
  ;[0.06618 0.2108 0.295] Sets up connections with the paired cable, as well as assigning any colours to the Model that it is intended to have
  (`parent.UserConstructionScript`)
  (`MeshComponent.SetVectorParameterValueOnMaterials` (`self.Model`) "Colour" (`KismetMathLibrary.Conv_LinearColorToVector` (`self.Colour`)))
  (if (and (`KismetSystemLibrary.IsValid` _cable_pair_reference) (`self.isCableHost?`))
    (bind _returnvalue (`AddComponent|NODE_AddCableComponent-0` :`RelativeTransform` (`KismetMathLibrary.MakeTransform` (.location (`SceneComponent.K2_GetComponentToWorld` (`self.Model`))) (.rotation (`SceneComponent.K2_GetComponentToWorld` (`self.Model`))))))
    (set `CableComponent.bAttachStart` true _returnvalue)
    (`CableComponent.SetAttachEndTo` _returnvalue _cable_pair_reference "Model" "None")
    (`SceneComponent.K2_SetWorldLocation` _returnvalue (`SceneComponent.K2_GetComponentLocation` (`self.Model`)) false false)
    (set `CableComponent.bEnableCollision` true _returnvalue)))